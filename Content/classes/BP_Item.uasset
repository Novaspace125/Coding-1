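; BP_Item is an item Blueprint that sets up its stats by type and automatically damages an enemy shortly after play begins.
; On BeginPlay a custom setup function switches on Type: weapons roll random damage and take a name from a shuffled list, while tools and consumables get fixed damage.
; It prints the result, waits briefly, then subtracts Damage from the Health of the Bp_enemy returned by GetActorOfClass, without a validity check.
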(event EventBeginPlay
  (CallFunction|Constuctor)
  (Development|PrintString (Utilities|String|Append "My damage = " (Variables|Default|GetName) " , damage " (Utilities|String|ToString(Integer) (Variables|Default|GetDamage))) true true "(R=0.000000,G=0.660000,B=1.000000,A=1.000000)" 1e+01)
  (Utilities|FlowControl|Delay 5.0)
  (bind _returnvalue (Actor|GetActorOfClass "/Game/blueprint/Bp_enemy.Bp_enemy_C"))
  (CallFunction|Attack _returnvalue))

(event Collision|EventActorBeginOverlap
  (params (OtherActor :type Actor%20Object%20Reference)))

(event EventTick
  (params (DeltaSeconds :type Float%20%28single-precision%29)))

(fn ConstructionScript)

(fn Constuctor
  (bind _weaponnames (Variables|Default|GetWeaponNames))
  (switch Utilities|FlowControl|Switch|SwitchonItemType (Variables|Default|GetType)
    (:NewEnumerator0
      (Variables|Default|SetDamage (Math|Random|RandomIntegerinRange 3 6))
      (if true ; If true randomize name\nif false, they alredy have a name
        (Utilities|Array|Shuffle _weaponnames) ; shuffle the list
        (Variables|Default|SetName (Utilities|Array|Get(acopy) _weaponnames)) ; set namer
      ))
    (:NewEnumerator1
      (Variables|Default|SetDamage 1))
    (:NewEnumerator2
      (Variables|Default|SetDamage 0))))

(fn Attack
  (params (Given%20enemy :type Bp%20Enemy%20Object%20Reference))
  (Variables|/Game/blueprint/Bp_enemy.Bp_enemy_C|SetHealth Given%20enemy (- (Variables|/Game/blueprint/Bp_enemy.Bp_enemy_C|GetHealth Given%20enemy) (Variables|Default|GetDamage))))