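; Enemy actor that dies when the player character touches it.
; CheckHealth starts on BeginPlay and re-calls itself after a short Delay, polling Health instead of reacting to changes, and destroys the actor once Health drops below zero.
; A Capsule overlap with BP_ThirdPersonCharacter sets Health negative, so the next poll removes the enemy.
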(event OnComponentBeginOverlap(Capsule)
  (params (OverlappedComponent :type Primitive%20Component%20Object%20Reference) (OtherActor :type Actor%20Object%20Reference) (OtherComp :type Primitive%20Component%20Object%20Reference) (OtherBodyIndex :type Integer) (bFromSweep :type Boolean) (SweepResult :type Hit%20Result%20Structure%20%28by%20ref%29))
  (Utilities|Casting|CastToBP_ThirdPersonCharacter OtherActor)
  (Variables|Default|SetHealth -1.0) ; search set health
)

(event Custom|Check%20Health
  (Utilities|FlowControl|Delay 0.2)
  (if (>= (Variables|Default|GetHealth) 0.0) ; If statmenr
    (CallFunction|CheckHealth) ; loop without rerouting
    (else
      (Actor|DestroyActor))))

(event EventBeginPlay
  (CallFunction|CheckHealth))

(fn ConstructionScript)