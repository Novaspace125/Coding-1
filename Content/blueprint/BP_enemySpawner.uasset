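; Enemy spawner actor that fills the level's spawn location markers with enemies and refills them whenever all enemies are gone.
; On BeginPlay it gathers every BP_enemySpawnLocation, prints the count, and spawns a Bp_enemy at each with an 80% chance.
; A self-recalling check with a Delay polls the number of live enemies every couple of seconds and triggers a new wave when it reaches zero.
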(event Custom|Spawn%20enemies
  (for _array_element (stale EventBeginPlay _outactors) ; better for loop, just tells the location
    (if (< (Math|Random|RandomFloat) 0.8) ; If statment
      (Game|SpawnActorfromClass "/Game/blueprint/Bp_enemy.Bp_enemy_C" (Transformation|GetActorTransform _array_element) "Undefined" "MultiplyWithRoot" 0 0) ; spawn from class\nspawns eneimy each loop
    )))

(event Custom|Check%20enemy%20check
  (bind _outactors (Actor|GetAllActorsOfClass "/Game/blueprint/Bp_enemy.Bp_enemy_C"))
  (if (> (Utilities|Array|Length _outactors) 0) ; falase spawns more enemies
    _
    (else
      (CallFunction|SpawnEnemies)))
  (Utilities|FlowControl|Delay 2.0)
  (CallFunction|CheckEnemyCheck))

(event EventBeginPlay
  (bind _outactors (Actor|GetAllActorsOfClass "/Game/blueprint/BP_enemySpawnLocation.BP_enemySpawnLocation_C")) ; put all of the location actor into an arrat
  (Development|PrintString (Utilities|String|Append "There are " (Utilities|String|ToString(Integer) (Utilities|Array|Length _outactors)) " spawn locations") true true "(R=0.000000,G=0.660000,B=1.000000,A=1.000000)" 1e+01)
  (CallFunction|SpawnEnemies)
  (CallFunction|CheckEnemyCheck))

(fn ConstructionScript)